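; UQ_CoinActor is a collectible coin that spins in place and adds to the player's score when picked up.
; On BeginPlay, a RotationZ timeline drives the Cylinder mesh's yaw while holding it upright at a 90-degree pitch.
; When an actor tagged Player overlaps SphereTrigger, it increments Score on ThirdPersonGameMode and destroys itself.
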(event `self.ReceiveBeginPlay`
  (bind (_direction _value) (`Timeline|RotationZ`)
    (:`Update`
      (`SceneComponent.K2_SetRelativeRotation` (`self.Cylinder`) (`KismetMathLibrary.MakeRotator` 0.0 90.0 _value) false false))))

(event `self.SphereTrigger.OnComponentBeginOverlap`
  (params (OverlappedComponent :type "PrimitiveComponent Object Reference") (OtherActor :type "Actor Object Reference") (OtherComp :type "PrimitiveComponent Object Reference") (OtherBodyIndex :type Integer) (bFromSweep :type Boolean) (SweepResult :type "HitResult Structure (by ref)"))
  (bind _asthird_person_game_mode (cast `/Game/ThirdPersonBP/Blueprints/ThirdPersonGameMode` (`GameplayStatics.GetGameMode`) :!pure true))
  (if (`self.ActorHasTag` OtherActor "Player")
    (set `/Game/ThirdPersonBP/Blueprints/ThirdPersonGameMode.Score` (+ (`/Game/ThirdPersonBP/Blueprints/ThirdPersonGameMode.Score` _asthird_person_game_mode) 1) _asthird_person_game_mode)
    (`self.K2_DestroyActor`)))

(fn `UserConstructionScript`)