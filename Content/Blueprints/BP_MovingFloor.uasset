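; BP_MovingFloor is a floor actor that travels at constant speed through an array of waypoint actors, looping or ping-ponging according to IsRoop.
; Construction and BeginPlay snap it to the first waypoint, then SetNewMoveLocation picks the next index and computes velocity.
; Tick moves it without sweep, detects arrival by comparing squared distances from the segment start, snaps to the target, then pauses on a timer before the next leg.
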(event `self.ReceiveBeginPlay`
  (set `self.MoveForward` true)
  (`self.K2_SetActorLocation` (`self.K2_GetActorLocation` (`|GetArrayItem` (`self.MoveRocations`))))
  (set `self.IndexMovingTo` 0)
  (`self.SetNewMoveLocation`))

(event `self.ReceiveTick`
  (params (DeltaSeconds :type "Float (single-precision)"))
  (bind _returnvalue (`self.K2_GetActorLocation` (`|GetArrayItem` (`self.MoveRocations`) (`self.IndexMovingFrom`))))
  (if (not (`self.Pausing`))
    (`self.K2_SetActorLocation` (+ (* (`self.velocity`) DeltaSeconds) (`self.K2_GetActorLocation`)))
    (if (>= (`KismetMathLibrary.VSizeSquared` (- (`self.K2_GetActorLocation`) _returnvalue)) (`KismetMathLibrary.VSizeSquared` (- _returnvalue (`self.K2_GetActorLocation` (`|GetArrayItem` (`self.MoveRocations`) (`self.IndexMovingTo`))))))
      (`self.K2_SetActorLocation` (`self.K2_GetActorLocation` (`|GetArrayItem` (`self.MoveRocations`) (`self.IndexMovingTo`))))
      (set `self.Pausing` true)
      (`KismetSystemLibrary.K2_SetTimer` null "SetNewMoveLocation" (`self.Interval`)))))

(fn `SetNewMoveLocation`
  (bind _moverocations (`self.MoveRocations`))
  (bind _indexmovingto (`self.IndexMovingTo`))
  (set `self.IndexMovingFrom` (`self.IndexMovingTo`))
  (if (`self.MoveForward`)
    (bind _result (`/Engine/EditorBlueprintResources/StandardMacros.IncrementInt` _indexmovingto)
      (:`  `
        (if (>= _result (`KismetArrayLibrary.Array_Length` (`self.MoveRocations`)))
          (if (`self.IsRoop`)
            (set `self.IndexMovingTo` 0)
            (else
              (set `self.MoveForward` false)
              (set `self.IndexMovingTo` (- (`self.IndexMovingFrom`) 1)))))))
    (else
      (bind _result_2 (`/Engine/EditorBlueprintResources/StandardMacros.DecrementInt` _indexmovingto)
        (:`  `
          (if (< _result_2 0)
            (set `self.MoveForward` true)
            (set `self.IndexMovingTo` (+ (`self.IndexMovingFrom`) 1)))))))
  (set `self.velocity` (* (`KismetMathLibrary.Normal` (- (`self.K2_GetActorLocation` (`|GetArrayItem` _moverocations (`self.IndexMovingTo`))) (`self.K2_GetActorLocation` (`|GetArrayItem` _moverocations (`self.IndexMovingFrom`))))) (`self.MoveSpeed`)))
  (set `self.Pausing` false))

(fn `UserConstructionScript`
  (`self.K2_SetActorLocation` (`self.K2_GetActorLocation` (`|GetArrayItem` (`self.MoveRocations`)))))