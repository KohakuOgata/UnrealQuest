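; Enemy actor that sweeps a rotating sight beam to spot the living player.
; Tick rotates the sight vector; DetectPlayer line-traces along it, snaps the beam particle to the result and returns player-alive status and seen actor.
; Chase, search and patrol events recolor eye and beam via dynamic materials, setting blink, sweep speed or state flags.
; Any damage ragdolls its parts, triggers an explosion, detaches the controller and adds score.
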(event `self.ReceiveBeginPlay`
  (set `self.Sight` (`KismetMathLibrary.MakeVector` (`self.SightRange`) 0.0 -100.0))
  (bind _returnvalue (`PrimitiveComponent.CreateDynamicMaterialInstance` (`self.Eye`) 0 "/Game/Materials/M_EnemyHeadBase.M_EnemyHeadBase" "None"))
  (bind _output_get (set `self.EyeDMI` _returnvalue))
  (`MaterialInstanceDynamic.SetVectorParameterValue` _output_get "Color" (`self.NormalEyeColor`))
  (`MaterialInstanceDynamic.SetScalarParameterValue` _output_get "BlinkCycle" (`self.NormalBeamRotateSpeed`))
  (bind _returnvalue_2 (`PrimitiveComponent.CreateDynamicMaterialInstance` (`self.P_Beam`) 0 "/Game/Materials/M_Beam.M_Beam" "None"))
  (bind _output_get_2 (set `self.BeamDMI` _returnvalue_2))
  (`MaterialInstanceDynamic.SetVectorParameterValue` _output_get_2 "Color" (`self.NormalEyeColor`))
  (set `self.BeamRotateSpeed` (`self.NormalBeamRotateSpeed`)))

(event `self.ReceiveHit`
  (params (MyComp :type "PrimitiveComponent Object Reference") (Other :type "Actor Object Reference") (OtherComp :type "PrimitiveComponent Object Reference") (bSelfMoved :type Boolean) (HitLocation :type "Vector Structure") (HitNormal :type "Vector Structure") (NormalImpulse :type "Vector Structure") (Hit :type "HitResult Structure (by ref)")))

(event `self.ReceiveTick`
  (params (DeltaSeconds :type "Float (single-precision)"))
  ;[0.07812 1 0] 索敵
  (set `self.Sight` (`KismetMathLibrary.RotateAngleAxis` (`self.Sight`) (* (* 360.0 DeltaSeconds) (`self.BeamRotateSpeed`)) (0.0 0.0 1.0))))

(event `self.ReceiveAnyDamage`
  (params (Damage :type "Float (single-precision)") (DamageType :type "DamageType Object Reference") (InstigatedBy :type "Controller Object Reference") (DamageCauser :type "Actor Object Reference"))
  (bind _eyedmi (`self.EyeDMI`))
  (bind _asthird_person_game_mode (cast `/Game/ThirdPersonBP/Blueprints/ThirdPersonGameMode` (`GameplayStatics.GetGameMode`) :!pure true))
  (`self.Set Simulate` (`self.Eye`))
  (`self.Set Simulate` (`self.Leg`))
  (`self.Set Simulate` (`self.Body`))
  (`self.Set Simulate` (`self.Head`))
  (`SceneComponent.SetVisibility` (`self.P_Beam`) false false)
  (`MaterialInstanceDynamic.SetVectorParameterValue` _eyedmi "Color" (struct :`R` 0.057292 :`G` 0.057292 :`B` 0.057292 :`A` 1.0))
  (`MaterialInstanceDynamic.SetScalarParameterValue` _eyedmi "BlinkCycle" 0.0)
  (`ActorComponent.SetActive` (`self.P_Explosion`) true false)
  (`KismetSystemLibrary.Delay` 0.01)
  (`self.DetachFromControllerPendingDestroy`)
  (`self.SetLifeSpan` 3.0)
  (set `/Game/ThirdPersonBP/Blueprints/ThirdPersonGameMode.Score` (+ (`/Game/ThirdPersonBP/Blueprints/ThirdPersonGameMode.Score` _asthird_person_game_mode) 5) _asthird_person_game_mode))

(event `BeginChace`
  (bind _eyedmi (`self.EyeDMI`))
  ;[1 0 0] プレイヤーを発見したとき
  (`MaterialInstanceDynamic.SetVectorParameterValue` _eyedmi "Color" (`self.ChacingEyeColor`))
  (`MaterialInstanceDynamic.SetScalarParameterValue` _eyedmi "BlinkCycle" (* (`self.NormalBeamRotateSpeed`) 4.0))
  (`MaterialInstanceDynamic.SetVectorParameterValue` (`self.BeamDMI`) "Color" (`self.ChacingEyeColor`))
  (set `self.PlayerDetected` true)
  (set `self.CanDamaged` false))

(event `BeginSerch`
  (bind _eyedmi (`self.EyeDMI`))
  (bind _serchingeyecolor (`self.SerchingEyeColor`))
  ;[1 1 0] プレイヤーを見失ったとき
  (set `self.BeamRotateSpeed` (* (`self.NormalBeamRotateSpeed`) 2.0))
  (`MaterialInstanceDynamic.SetVectorParameterValue` _eyedmi "Color" _serchingeyecolor)
  (`MaterialInstanceDynamic.SetScalarParameterValue` _eyedmi "BlinkCycle" (`self.BeamRotateSpeed`))
  (`MaterialInstanceDynamic.SetVectorParameterValue` (`self.BeamDMI`) "Color" _serchingeyecolor)
  (set `self.CanDamaged` true))

(event `BeginPatrol`
  (bind _normaleyecolor (`self.NormalEyeColor`))
  (bind _eyedmi (`self.EyeDMI`))
  ;[0 1 1] プレイヤーの捜索を終了したとき
  (`MaterialInstanceDynamic.SetVectorParameterValue` _eyedmi "Color" _normaleyecolor)
  (`MaterialInstanceDynamic.SetScalarParameterValue` _eyedmi "BlinkCycle" (`self.NormalBeamRotateSpeed`))
  (`MaterialInstanceDynamic.SetVectorParameterValue` (`self.BeamDMI`) "Color" _normaleyecolor)
  (set `self.BeamRotateSpeed` (`self.NormalBeamRotateSpeed`))
  (set `self.CanDamaged` true))

(fn `DetectPlayer`
  (returns (ReturnValue :type Boolean) (SeenActor :type "Actor Object Reference"))
  (locals (HitActor :type "Actor Object Reference") (IsAlivePlayer :type Boolean))
  (bind _returnvalue (+ (`self.Sight`) (`SceneComponent.K2_GetComponentLocation` (`self.Head`))))
  (bind (_ishit _outhit) (`self.LineTrace` _returnvalue))
  (if _ishit
    (bind (_bblockinghit _binitialoverlap _time _distance _location _impactpoint _normal _impactnormal _physmat _hitactor) (`GameplayStatics.BreakHitResult` _outhit))
    (set `local.HitActor` _hitactor)
    (bind (_asthird_person_character _bsuccess) (cast `/Game/ThirdPersonBP/Blueprints/ThirdPersonCharacter` _hitactor :!pure true))
    (if _bsuccess
      (set `local.IsAlivePlayer` (`/Game/ThirdPersonBP/Blueprints/ThirdPersonCharacter.IsAlive` _asthird_person_character)))
    (`self.SetBeamPerticleTarget` _location)
    (else
      (`self.SetBeamPerticleTarget` _returnvalue)))
  (return (`local.IsAlivePlayer`) (`local.HitActor`)))

(fn `LineTrace`
  (params (EndLocation :type "Vector Structure"))
  (returns (IsHit :type Boolean) (OutHit :type "HitResult Structure"))
  (locals (HitReturn :type "HitResult Structure"))
  (bind (_outhit _returnvalue) (`KismetSystemLibrary.LineTraceSingle` (`SceneComponent.K2_GetComponentLocation` (`self.Head`)) EndLocation "TraceTypeQuery2"))
  (if _returnvalue
    (set `local.HitReturn` _outhit))
  (return _returnvalue (`local.HitReturn`)))

(fn `Set Simulate`
  (params (TargetMesh :type "StaticMeshComponent Object Reference"))
  (`PrimitiveComponent.SetSimulatePhysics` TargetMesh true)
  (`PrimitiveComponent.SetCollisionProfileName` TargetMesh "RagDoll" true))

(fn `SetBeamPerticleTarget`
  (params (NewTargetPoint :type "Vector Structure"))
  (`ParticleSystemComponent.SetBeamTargetPoint` (`self.P_Beam`) 0 NewTargetPoint 0))

(fn `UserConstructionScript`
  (`ParticleSystemComponent.SetBeamTargetPoint` (`self.P_Beam`) 0 (+ (`KismetMathLibrary.MakeVector` (`self.SightRange`) 0.0 -100.0) (`SceneComponent.K2_GetComponentLocation` (`self.Head`))) 0))